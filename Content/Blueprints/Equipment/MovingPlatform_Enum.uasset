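; Moving platform that a linked pressure switch starts, carrying its mesh back and forth along a spline.
; On BeginPlay it binds to the switch's pressed and released events, which share one mode check with only Activate on Pressed implemented.
; A timeline scaled by Duration drives spline distance and optional rotation, flipping direction on finish to ping-pong endlessly.
; The construction script applies the platform material.
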(event Custom|SwitchPressed
  (bind _spline (Variables|Default|GetSpline))
  (bind _staticmesh (Variables|Default|GetStaticMesh))
  (switch Utilities|FlowControl|Switch|SwitchonPressureSwitchModes (Variables|Default|GetPressureSwitchMode)
    (:NewEnumerator0
      (Components|Timeline|SetPlayRate (Variables|Default|GetMovePlatformTimeline) (/ 1.0 (Variables|Default|GetDuration)))
      (bind (_direction _traveldistance) (Timeline|MovePlatformTimeline Play)
        (:Update
          (Transformation|SetWorldLocation _staticmesh (Spline|GetLocationatDistanceAlongSpline _spline (* _traveldistance (Spline|GetSplineLength _spline)) "World") false false)
          (if (Variables|Default|GetModifyRotation?)
            (Transformation|SetRelativeRotation _staticmesh (Spline|GetRotationatDistanceAlongSpline _spline (* _traveldistance (Spline|GetSplineLength _spline)) "Local") false false)))
        (:Finished
          (switch Utilities|FlowControl|Switch|SwitchonETimelineDirection _direction
            (:Forward
              (Timeline|MovePlatformTimeline Reverse))
            (:Backward
              (Timeline|MovePlatformTimeline Play))))))))

(event Custom|SwitchReleased
  (bind _spline (Variables|Default|GetSpline))
  (bind _staticmesh (Variables|Default|GetStaticMesh))
  (switch Utilities|FlowControl|Switch|SwitchonPressureSwitchModes (Variables|Default|GetPressureSwitchMode)
    (:NewEnumerator0
      (Components|Timeline|SetPlayRate (Variables|Default|GetMovePlatformTimeline) (/ 1.0 (Variables|Default|GetDuration)))
      (bind (_direction _traveldistance) (Timeline|MovePlatformTimeline Play)
        (:Update
          (Transformation|SetWorldLocation _staticmesh (Spline|GetLocationatDistanceAlongSpline _spline (* _traveldistance (Spline|GetSplineLength _spline)) "World") false false)
          (if (Variables|Default|GetModifyRotation?)
            (Transformation|SetRelativeRotation _staticmesh (Spline|GetRotationatDistanceAlongSpline _spline (* _traveldistance (Spline|GetSplineLength _spline)) "Local") false false)))
        (:Finished
          (switch Utilities|FlowControl|Switch|SwitchonETimelineDirection _direction
            (:Forward
              (Timeline|MovePlatformTimeline Reverse))
            (:Backward
              (Timeline|MovePlatformTimeline Play))))))))

(event EventBeginPlay
  (bind _pressureswitchreference (Variables|Default|GetPressureSwitchReference))
  (Utilities|IsValid _pressureswitchreference
    (:Is%20Valid
      (EventDispatchers|BindEventtoSwitchPressed _pressureswitchreference (delegate Custom|SwitchPressed))
      (EventDispatchers|BindEventtoSwitchReleased (Variables|Default|GetPressureSwitchReference) (delegate Custom|SwitchReleased)))))

(fn ConstructionScript
  (Rendering|Material|SetMaterial (Variables|Default|GetStaticMesh) 0 (Variables|Default|GetPlatformMaterial)))