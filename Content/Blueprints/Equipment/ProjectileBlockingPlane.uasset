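; Equipment plane that blocks or destroys a configured projectile class, and can also block pawns.
; An optional pressure switch toggles its visibility and active state on press or release through DoOnce anti-flicker gates; without a switch it starts active.
; A Box overlap pre-screens incoming actors, either arming destruction with a particle on Plane overlap or switching the Plane's projectile channel between Block and Overlap, which Plane hits also re-evaluate.
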(event OnComponentBeginOverlap(Box)
  (params (OverlappedComponent :type Primitive%20Component%20Object%20Reference) (OtherActor :type Actor%20Object%20Reference) (OtherComp :type Primitive%20Component%20Object%20Reference) (OtherBodyIndex :type Integer) (bFromSweep :type Boolean) (SweepResult :type Hit%20Result%20Structure%20%28by%20ref%29))
  ;[1 1 1] Handles destruction of projectiles when set to overlap, allows switch to a blocking volume
  (if (Math|Boolean|ANDBoolean (Variables|Default|GetDestroyProjectileOnCollision?) (Variables|Default|GetIsPlaneActive?) (Utilities|ClassIsChildOf (Utilities|GetClass OtherActor) (Variables|Default|GetBlockingProjectile)))
    (Variables|Default|SetProjectileKillOnPlaneCollision true)
    (else
      (CallFunction|ProjectileCollisionandDestructionTest OtherActor) ; This sends non-matching projectiles into a function that changes the collision settings of the plane
    )))

(event OnComponentHit(Plane)
  (params (HitComponent :type Primitive%20Component%20Object%20Reference) (OtherActor :type Actor%20Object%20Reference) (OtherComp :type Primitive%20Component%20Object%20Reference) (NormalImpulse :type Vector :default "0, 0, 0") (Hit :type Hit%20Result%20Structure%20%28by%20ref%29))
  ;[1 1 1] Handles logic for when plane becomes a blocking volume for projectiles
  (if (Utilities|ClassIsChildOf (Utilities|GetClass OtherActor) "/Game/Blueprints/Weapons/Projectiles/FirstPersonProjectile.FirstPersonProjectile_C")
    (CallFunction|ProjectileCollisionandDestructionTest OtherActor)))

(event OnComponentBeginOverlap(Plane)
  (params (OverlappedComponent :type Primitive%20Component%20Object%20Reference) (OtherActor :type Actor%20Object%20Reference) (OtherComp :type Primitive%20Component%20Object%20Reference) (OtherBodyIndex :type Integer) (bFromSweep :type Boolean) (SweepResult :type Hit%20Result%20Structure%20%28by%20ref%29))
  (if (and (Variables|Default|GetProjectileKillOnPlaneCollision) (Utilities|ClassIsChildOf (Utilities|GetClass 0) (Variables|Default|GetBlockingProjectile)))
    (bind _asfirst_person_projectile (Utilities|Casting|CastToFirstPersonProjectile OtherActor))
    (Effects|SpawnEmitteratLocation "/Game/Materials/PBP_Particle.PBP_Particle" (Transformation|GetActorLocation _asfirst_person_projectile))
    (Actor|DestroyActor OtherActor) ; destroys matching projectiles
  ))

(event Custom|SwitchPressed
  (Variables|Default|SetIsButtonPressed? true)
  ;[1 1 1] This is a gate to prevent flickering
  (Utilities|FlowControl|Sequence
    (:then_0
      (Utilities|FlowControl|DoOnce false
        (:Completed
          (CallFunction|PressureSwitchLogic (Variables|Default|GetPressureSwitchMode)))))
    (:then_1
      (Utilities|FlowControl|DoOnce false) ; enters at Reset
    )))

(event Custom|SwitchReleased
  (Variables|Default|SetIsButtonPressed? false)
  ;[1 1 1] This is a gate to prevent flickering
  (Utilities|FlowControl|Sequence
    (:then_0
      (Utilities|FlowControl|DoOnce false
        (:Completed
          (CallFunction|PressureSwitchLogic (Variables|Default|GetPressureSwitchMode)))))
    (:then_1
      (Utilities|FlowControl|DoOnce false) ; enters at Reset
    )))

(event EventBeginPlay
  (bind _pressureswitchreference (Variables|Default|GetPressureSwitchReference))
  (Utilities|IsValid (Variables|Default|GetPressureSwitchReference)
    (:Is%20Valid
      (EventDispatchers|BindEventtoSwitchPressed _pressureswitchreference (delegate Custom|SwitchPressed))
      (EventDispatchers|BindEventtoSwitchReleased _pressureswitchreference (delegate Custom|SwitchReleased))
      (CallFunction|PressureSwitchLogic (Variables|Default|GetPressureSwitchMode)))
    (:Is%20Not%20Valid
      (bind _output_get (Variables|Default|SetPressureSwitchMode "NewEnumerator1"))
      (CallFunction|PressureSwitchLogic _output_get))))

(event EventTick
  (params (DeltaSeconds :type Float%20%28single-precision%29)))

(fn ConstructionScript)

(fn PressureSwitchLogic
  (params (PressureSwitchMode :type PressureSwitchModes%20Enum :default "NewEnumerator0"))
  (bind _isbuttonpressed_ (Variables|Default|GetIsButtonPressed?))
  (switch Utilities|FlowControl|Switch|SwitchonPressureSwitchModes PressureSwitchMode
    (:NewEnumerator0
      (CallFunction|PressureSwitchVisual _isbuttonpressed_))
    (:NewEnumerator1
      (CallFunction|PressureSwitchVisual (not _isbuttonpressed_)))))

(fn PressureSwitchVisual
  (params (IsButtonPressed? :type Boolean))
  (bind _plane (Variables|Default|GetPlane))
  (bind _output_get (LocalVariables|SetLocalButtonPressed IsButtonPressed?))
  (if _output_get
    (Rendering|SetVisibility (Variables|Default|GetPlane) (LocalVariables|GetLocalButtonPressed) false)
    (Variables|Default|SetIsPlaneActive? true)
    (else
      (Rendering|SetVisibility (Variables|Default|GetPlane) (LocalVariables|GetLocalButtonPressed) false)
      (Variables|Default|SetIsPlaneActive? false)))
  (if (and (Variables|Default|GetIsPlaneActive?) (Variables|Default|GetBlockPlayer?))
    (Collision|SetCollisionResponsetoChannel _plane "ECC_Pawn" "ECR_Block")
    (else
      (Collision|SetCollisionResponsetoChannel _plane "ECC_Pawn" "ECR_Overlap"))))

(fn ProjectileCollisionandDestructionTest
  (params (Other%20Actor :type Actor%20Object%20Reference))
  (bind _plane (Variables|Default|GetPlane))
  (if (and (Variables|Default|GetIsPlaneActive?) (Utilities|ClassIsChildOf (Utilities|GetClass Other%20Actor) (Variables|Default|GetBlockingProjectile)))
    (Collision|SetCollisionResponsetoChannel _plane "ECC_GameTraceChannel1" "ECR_Block")
    (else
      (Collision|SetCollisionResponsetoChannel _plane "ECC_GameTraceChannel1" "ECR_Overlap"))))