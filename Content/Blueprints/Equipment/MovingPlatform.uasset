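; Moving platform that shuttles a static mesh back and forth along a spline, controlled by a referenced pressure switch.
; ButtonActivatesMovement selects whether pressing or releasing the switch triggers movement through a DoOnce, which resets only on release in press-to-move mode.
; A timeline, rate-scaled by Duration, drives distance along the spline and optional rotation, reversing at each end.
; The construction script applies the platform material.
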(event Custom|SwitchPressed
  (bind _spline (Variables|Default|GetSpline))
  (bind _staticmesh (Variables|Default|GetStaticMesh))
  (if (Variables|Default|GetButtonActivatesMovement?)
    (Components|Timeline|SetPlayRate (Variables|Default|GetMovePlatformTimeline) (/ 1.0 (Variables|Default|GetDuration)))
    (Utilities|FlowControl|DoOnce false
      (:Completed
        (bind (_direction _traveldistance) (Timeline|MovePlatformTimeline Play)
          (:Update
            (Transformation|SetWorldLocation _staticmesh (Spline|GetLocationatDistanceAlongSpline _spline (* _traveldistance (Spline|GetSplineLength _spline)) "World") false false)
            (if (Variables|Default|GetModifyRotation?)
              (Transformation|SetRelativeRotation _staticmesh (Spline|GetRotationatDistanceAlongSpline _spline (* _traveldistance (Spline|GetSplineLength _spline)) "Local") false false)))
          (:Finished
            (switch Utilities|FlowControl|Switch|SwitchonETimelineDirection _direction
              (:Forward
                (Timeline|MovePlatformTimeline Reverse))
              (:Backward
                (Timeline|MovePlatformTimeline Play)))))))
    (else
      (Timeline|MovePlatformTimeline Stop))))

(event Custom|SwitchReleased
  (bind _spline (Variables|Default|GetSpline))
  (bind _staticmesh (Variables|Default|GetStaticMesh))
  (if (Variables|Default|GetButtonActivatesMovement?)
    (Utilities|FlowControl|Sequence
      (:then_0
        (goto _label Reset))
      (:then_1
        (bind (_direction _traveldistance) (Timeline|MovePlatformTimeline Stop)
          (:Update
            (Transformation|SetWorldLocation _staticmesh (Spline|GetLocationatDistanceAlongSpline _spline (* _traveldistance (Spline|GetSplineLength _spline)) "World") false false)
            (if (Variables|Default|GetModifyRotation?)
              (Transformation|SetRelativeRotation _staticmesh (Spline|GetRotationatDistanceAlongSpline _spline (* _traveldistance (Spline|GetSplineLength _spline)) "Local") false false)))
          (:Finished
            (switch Utilities|FlowControl|Switch|SwitchonETimelineDirection _direction
              (:Forward
                (Timeline|MovePlatformTimeline Reverse))
              (:Backward
                (Timeline|MovePlatformTimeline Play)))))))
    (else
      (Components|Timeline|SetPlayRate (Variables|Default|GetMovePlatformTimeline) (/ 1.0 (Variables|Default|GetDuration)))
      (Utilities|FlowControl|DoOnce false :!label _label
        (:Completed
          (Timeline|MovePlatformTimeline Play))))))

(event EventBeginPlay
  (EventDispatchers|BindEventtoSwitchPressed (Variables|Default|GetPressureSwitchReference) (delegate Custom|SwitchPressed))
  (EventDispatchers|BindEventtoSwitchReleased (Variables|Default|GetPressureSwitchReference) (delegate Custom|SwitchReleased)))

(fn ConstructionScript
  (Rendering|Material|SetMaterial (Variables|Default|GetStaticMesh) 0 (Variables|Default|GetPlatformMaterial)))