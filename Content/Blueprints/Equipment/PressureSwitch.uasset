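; Pressure switch actor that signals when it is pressed or released by overlapping objects.
; Trigger overlap events keep a count of objects on the switch and store the latest actor reference, clearing it on any exit.
; Tick polls the count, sinks the plate and calls pressed every frame while occupied.
; When empty it raises the plate, and a DoOnce, reset while pressed, limits the released call to once.
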(event OnComponentBeginOverlap(SwitchTrigger)
  (params (OverlappedComponent :type Primitive%20Component%20Object%20Reference) (OtherActor :type Actor%20Object%20Reference) (OtherComp :type Primitive%20Component%20Object%20Reference) (OtherBodyIndex :type Integer) (bFromSweep :type Boolean) (SweepResult :type Hit%20Result%20Structure%20%28by%20ref%29))
  (Variables|Default|SetOtherActorReference OtherActor)
  (Math|Integer|IncrementInt (Variables|Default|GetNumberOfObjects)))

(event OnComponentEndOverlap(SwitchTrigger)
  (params (OverlappedComponent :type Primitive%20Component%20Object%20Reference) (OtherActor :type Actor%20Object%20Reference) (OtherComp :type Primitive%20Component%20Object%20Reference) (OtherBodyIndex :type Integer))
  (Variables|Default|SetOtherActorReference 0)
  (Math|Integer|DecrementInt (Variables|Default|GetNumberOfObjects)))

(event EventBeginPlay)

(event Collision|EventActorBeginOverlap
  (params (OtherActor :type Actor%20Object%20Reference)))

(event EventTick
  (params (DeltaSeconds :type Float%20%28single-precision%29))
  (if (>= (Variables|Default|GetNumberOfObjects) 1)
    (Default|CallSwitchPressed)
    (Transformation|SetRelativeLocation (Variables|Default|GetPressureSwitch) "0, 0,-10.000000" false false)
    (goto _label Reset)
    (else
      (Transformation|SetRelativeLocation (Variables|Default|GetPressureSwitch) "0, 0,-5.000000" false false)
      (Utilities|FlowControl|DoOnce false :!label _label
        (:Completed
          (Default|CallSwitchReleased))))))

(fn ConstructionScript)