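; Equipment actor that acts as a switch-controlled barrier against teleport projectiles.
; It binds to the pressed and released events of a referenced pressure switch, which set and clear its active state.
; Pressing shows the plane if hidden, while releasing toggles its visibility without checking the current state.
; While active, any TeleportProjectile that begins overlapping the actor is destroyed.
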(event Custom|SwitchPressed
  (bind _plane (Variables|Default|GetPlane))
  (Variables|Default|SetIsActive? true)
  (if (not (Rendering|IsVisible _plane))
    (Rendering|ToggleVisibility _plane false)))

(event Custom|SwitchReleased
  (Variables|Default|SetIsActive? false)
  (Rendering|ToggleVisibility (Variables|Default|GetPlane) false))

(event EventBeginPlay
  (bind _pressureswitchreference (Variables|Default|GetPressureSwitchReference))
  (EventDispatchers|BindEventtoSwitchPressed _pressureswitchreference (delegate Custom|SwitchPressed))
  (EventDispatchers|BindEventtoSwitchReleased _pressureswitchreference (delegate Custom|SwitchReleased)))

(event Collision|EventActorBeginOverlap
  (params (OtherActor :type Actor%20Object%20Reference))
  (if (Variables|Default|GetIsActive?)
    (bind _asteleport_projectile (Utilities|Casting|CastToTeleportProjectile OtherActor))
    (Actor|DestroyActor _asteleport_projectile)))

(event EventTick
  (params (DeltaSeconds :type Float%20%28single-precision%29)))

(fn ConstructionScript)