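; Test weapon Blueprint that fires a single projectile, then teleports the player to that projectile's stored location on scope input.
; TestShoot spawns the projectile aimed at the camera target, adds half the player's velocity, and saves references both ways.
; ScopeBegin teleports and destroys the projectile when ShotCounter is one; this file never resets the counter.
; Tick prints the counter for debugging.
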(event EventBeginPlay
  (|CallParentFunction) ; This node is disabled and will not be called.\nDrag off pins to build functionality.
)

(event Collision|EventActorBeginOverlap
  (params (OtherActor :type Actor%20Object%20Reference)))

(event EventTick
  (params (DeltaSeconds :type Float%20%28single-precision%29))
  (|CallParentFunction DeltaSeconds)
  (Development|PrintString (Utilities|String|ToString(Integer) (Variables|Default|GetShotCounter)) true true "(R=0.000000,G=0.660000,B=1.000000,A=1.000000)" DeltaSeconds))

(event EventShoot
  (CallFunction|TestShoot))

(event EventScopeBegin
  (if (== (Variables|Default|GetShotCounter) 1)
    (bind _astest_projectile (Utilities|Casting|CastToTestProjectile (Variables|Default|GetProjectileReference))
      (:then
        (Transformation|Teleport (Game|GetPlayerCharacter 0) (Variables|/Game/Blueprints/Weapons/Projectiles/TestProjectile.TestProjectile_C|GetTeleportLocation _astest_projectile) "0, 0, 0")
        (Actor|DestroyActor (Variables|Default|GetProjectileReference))
        (Variables|Default|SetProjectileReference 0))
      (:CastFailed
        (Development|PrintString ":(")))
    (else
      (Development|PrintString "Can't Teleport"))))

(fn ConstructionScript
  (|CallParentFunction))

(fn TestShoot
  (bind _projectilespawn (Variables|Default|GetProjectileSpawn))
  (bind _returnvalue (Transformation|GetWorldLocation _projectilespawn))
  (bind _location (Default|GetCameraTarget (Variables|Default|Getplayer)))
  (if (< (Variables|Default|GetShotCounter) 1)
    (bind _returnvalue_2 (Game|SpawnActorfromClass (Variables|Default|GetProjectileType) (Math|Transform|MakeTransform _returnvalue (Math|Rotator|FindLookatRotation _returnvalue _location) "1,1,1") "Undefined" 0 (Variables|Default|Getplayer)))
    (Variables|Default|SetProjectileReference _returnvalue_2)
    (Math|Integer|IncrementInt (Variables|Default|GetShotCounter)
      (:%20%20
        (Variables|/Game/Blueprints/Weapons/Projectiles/FirstPersonProjectile.FirstPersonProjectile_C|SetWeaponReference _returnvalue_2 self)
        ;[1 1 1] Inherit Velocity from Player
        (Variables|/Script/Engine.MovementComponent|SetVelocity (Variables|/Game/Blueprints/Weapons/Projectiles/FirstPersonProjectile.FirstPersonProjectile_C|GetProjectile _returnvalue_2) (+ (Variables|/Script/Engine.MovementComponent|GetVelocity (Variables|/Game/Blueprints/Weapons/Projectiles/FirstPersonProjectile.FirstPersonProjectile_C|GetProjectile _returnvalue_2)) (* (Transformation|GetVelocity (Game|GetPlayerCharacter 0)) 0.5)))
        (Audio|PlaySoundatLocation (Variables|Default|GetSoundShoot) (Transformation|GetActorLocation) "0, 0, 0" 1.0 1.0 0.0 0 0 0) ; Play firing sound
        (Variables|Default|SethasShot true)
        (Variables|Default|SetshootCooldownTimer (Variables|Default|GetshootCooldown))
        (Default|PayFireAnimation (Variables|Default|Getplayer))
        (return false)))))