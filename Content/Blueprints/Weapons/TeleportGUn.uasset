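; Teleport gun that launches a projectile the player can teleport to.
; TriggerPull shoots when no TeleportProjectile exists in the world, otherwise destroys the existing one with an airburst effect and sound.
; AbilityCall teleports player character 0 to the projectile, destroys it and starts a cooldown, playing click sounds when unavailable.
; Tick accumulates the cooldown, re-enabling teleport only when the timer nearly equals CooldownLimit within a small tolerance.
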(event EventBeginPlay
  (|CallParentFunction) ; This node is disabled and will not be called.\nDrag off pins to build functionality.
)

(event Collision|EventActorBeginOverlap
  (params (OtherActor :type Actor%20Object%20Reference)))

(event EventTick
  (params (DeltaSeconds :type Float%20%28single-precision%29))
  (|CallParentFunction DeltaSeconds)
  (if (not (Variables|Default|GetHasNotTeleported))
    (Variables|Default|SetCooldownTimer (+ DeltaSeconds (Variables|Default|GetCooldownTimer)))
    (if (Math|Float|NearlyEqual(Float) (Variables|Default|GetCooldownTimer) (Variables|Default|GetCooldownLimit) 0.01)
      (Variables|Default|SetCooldownTimer 0.0)
      (Variables|Default|SetHasNotTeleported true))))

(event EventTriggerPull
  (params (Player :type First%20Person%20Character%20Object%20Reference))
  (Variables|Default|Setplayer Player)
  (bind _outactors (Actor|GetAllActorsOfClass "/Game/Blueprints/Weapons/Projectiles/TeleportProjectile.TeleportProjectile_C"))
  (if (< (Utilities|Array|Length _outactors) 1)
    (CallFunction|Shoot)
    (else
      (Utilities|IsValid (Utilities|Array|Get(acopy) _outactors)
        (:Is%20Valid
          (Effects|SpawnEmitteratLocation "/Game/Particles/TeleportPelletAirburst.TeleportPelletAirburst" (Transformation|GetActorLocation (Utilities|Array|Get(acopy) _outactors)))
          (Actor|DestroyActor (Utilities|Array|Get(acopy) _outactors))
          (Audio|PlaySoundatLocation "/Engine/VREditor/Sounds/VR_negative_Cue.VR_negative_Cue" (Transformation|GetActorLocation) "0, 0, 0" 1.0 1.0 0.0 0 0 0))
        (:Is%20Not%20Valid
          (Development|PrintString "Failure validation of projectile for destruction"))))))

(fn ConstructionScript
  (|CallParentFunction))

(fn AbilityCall
  (bind _returnvalue (Game|GetPlayerCharacter 0))
  (bind _outactors (Actor|GetAllActorsOfClass "/Game/Blueprints/Weapons/Projectiles/TeleportProjectile.TeleportProjectile_C"))
  (Utilities|IsValid (Utilities|Array|Get(acopy) _outactors)
    (:Is%20Valid
      (if (Variables|Default|GetHasNotTeleported)
        (Transformation|Teleport _returnvalue (Transformation|GetActorLocation (Utilities|Array|Get(acopy) _outactors)) "0, 0, 0")
        (Audio|PlaySoundatLocation "/Engine/VREditor/Sounds/VR_teleport_Cue.VR_teleport_Cue" (Transformation|GetActorLocation _returnvalue) "0, 0, 0" 1.0 1.0 0.0 0 0 0)
        (Actor|DestroyActor (Utilities|Array|Get(acopy) _outactors))
        (Variables|Default|SetHasNotTeleported false)
        (else
          (Audio|PlaySoundatLocation "/Engine/VREditor/Sounds/VR_click1_Cue.VR_click1_Cue" "0, 0, 0" "0, 0, 0" 1.0 1.0 0.0 0 0 0))))
    (:Is%20Not%20Valid
      (Audio|PlaySoundatLocation "/Engine/VREditor/Sounds/VR_click2_Cue.VR_click2_Cue" "0, 0, 0" "0, 0, 0" 1.0 1.0 0.0 0 0 0))))