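; Teleport weapon that fires a projectile and can move the player to it when the trigger is held.
; Tick counts down the shot cooldown, calls Shoot on trigger press or plays a click while cooling down, and tracks hold time.
; With UseM1Teleport, hold time nearly equalling TeleportCooldown teleports the player to the first projectile found, destroys it and restarts the cooldown.
; An unconnected CanPlayerTeleport branch and a debug print remain.
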(event EventBeginPlay
  (|CallParentFunction))

(event Collision|EventActorBeginOverlap
  (params (OtherActor :type Actor%20Object%20Reference)))

(event EventTick
  (params (DeltaSeconds :type Float%20%28single-precision%29))
  (bind _returnvalue (Game|GetPlayerCharacter 0))
  (Utilities|FlowControl|Sequence
    (:then_0
      (Development|PrintString (Utilities|String|ToString(Float) (Variables|Default|GetTriggerHeldTime)) true true "(R=0.000000,G=0.660000,B=1.000000,A=1.000000)" DeltaSeconds)
      (if (> (Variables|Default|GetshootCooldownTimer) 0.0)
        (Variables|Default|SetshootCooldownTimer (- (Variables|Default|GetshootCooldownTimer) (Utilities|Time|GetWorldDeltaSeconds)))
        (if (and (Variables|Default|GetisTriggerPulled) (!= (Variables|Default|GetshootCooldownTimer) 0.0))
          (Utilities|FlowControl|DoOnce false :!label _label
            (:Completed
              (Audio|PlaySoundatLocation "/Engine/VREditor/Sounds/VR_click1_Cue.VR_click1_Cue" (Transformation|GetActorLocation) "0, 0, 0" 1.0 1.0 0.0 0 0 0)))
          (else
            (goto _label Reset)))
        (elif (Variables|Default|GetisTriggerPulled)
          (Utilities|FlowControl|DoOnce false :!label _label_2
            (:Completed
              (if (and (or (not (Variables|Default|GethasShot)) (Variables|Default|GetisAutomatic)) (not (Variables|Default|GetHasPlayerTeleported?)))
                (CallFunction|Shoot))))
          (else
            (goto _label_2 Reset)))))
    (:then_1
      (if (Variables|Default|GetisTriggerPulled)
        (Variables|Default|SetTriggerHeldTime (+ (Variables|Default|GetTriggerHeldTime) (Utilities|Time|GetWorldDeltaSeconds)))
        (else
          (Variables|Default|SetTriggerHeldTime 0.0))))
    (:then_2
      (if (and (Math|Float|NearlyEqual(Float) (Variables|Default|GetTriggerHeldTime) (Variables|Default|GetTeleportCooldown) 0.01) (Variables|Default|GetUseM1Teleport))
        (bind _outactors (Actor|GetAllActorsOfClass "/Game/Blueprints/Weapons/Projectiles/FirstPersonProjectile.FirstPersonProjectile_C"))
        (bind _asteleport_projectile (Utilities|Casting|CastToTeleportProjectile (Utilities|Array|Get(acopy) _outactors)))
        (Audio|PlaySoundatLocation "/Engine/VREditor/Sounds/UI/Teleport_Committed.Teleport_Committed" (Transformation|GetActorLocation) "0, 0, 0" 1.0 1.0 0.0 0 0 0)
        (Transformation|Teleport _returnvalue (Transformation|GetActorLocation _asteleport_projectile) (Transformation|GetActorRotation _returnvalue))
        (Actor|DestroyActor _asteleport_projectile)
        (Variables|Default|SetshootCooldownTimer 2.0)))))

(fn ConstructionScript
  (|CallParentFunction))