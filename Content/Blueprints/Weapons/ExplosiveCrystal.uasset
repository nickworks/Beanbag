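; ExplosiveCrystal is a weapon actor that grows into the world and removes itself after a short random lifespan.
; On BeginPlay it takes a random yaw with a slight random pitch, then a Grow timeline drives its uniform scale.
; Tick counts the lifespan down to destruction, and a hit from a FirstPersonProjectile destroys it early.
; Despite the name, this graph contains no explosion or damage logic.
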(event EventBeginPlay
  (bind _returnvalue (Math|Random|RandomRotator false))
  (Variables|Default|Setlifespan (Math|Random|RandomFloatinRange 1e+01 12.0))
  (Transformation|SetActorRotation (Math|Rotator|MakeRotator 0.0 (* (.pitch _returnvalue) 0.05) (.yaw _returnvalue)) true)
  (bind _scale (Timeline|Grow Play)
    (:Update
      (Transformation|SetActorScale3D (Math|Vector|MakeVector _scale _scale _scale)))))

(event EventTick
  (params (DeltaSeconds :type Float%20%28single-precision%29))
  (bind _output_get (Variables|Default|Setlifespan (- (Variables|Default|Getlifespan) DeltaSeconds)))
  (if (<= _output_get 0.0)
    (Actor|DestroyActor)))

(event Collision|EventHit
  (params (MyComp :type Primitive%20Component%20Object%20Reference) (Other :type Actor%20Object%20Reference) (OtherComp :type Primitive%20Component%20Object%20Reference) (bSelfMoved :type Boolean) (HitLocation :type Vector :default "0, 0, 0") (HitNormal :type Vector :default "0, 0, 0") (NormalImpulse :type Vector :default "0, 0, 0") (Hit :type Hit%20Result%20Structure%20%28by%20ref%29))
  (Utilities|Casting|CastToFirstPersonProjectile Other)
  (Actor|DestroyActor))

(fn ConstructionScript)