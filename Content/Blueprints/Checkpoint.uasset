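; Checkpoint actor that sets the player's respawn point and jetpack boost capacity on overlap.
; An overlapping FirstPersonCharacter gets its BoostFuelMax set from SecondsOfBoost, and the Arrow's location and rotation become BeanbagGameMode's SpawnTransform at unit scale.
; Tick compares the Arrow transform to that SpawnTransform, showing the particle system only on the active checkpoint.
; The overlap's own visibility check compares SpawnTransform to itself, so it always passes.
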(event EventBeginPlay)

(event Collision|EventActorBeginOverlap
  (params (OtherActor :type Actor%20Object%20Reference))
  (bind _arrow (Variables|Default|GetArrow))
  (bind _returnvalue (Transformation|GetWorldTransform _arrow))
  (bind _asfirst_person_character (Utilities|Casting|CastToFirstPersonCharacter OtherActor))
  (Variables|/Game/Blueprints/Equipment/JetpackComponent.JetpackComponent_C|SetboostFuelMax (Variables|/Game/Blueprints/FirstPersonCharacter.FirstPersonCharacter_C|GetJetpackComponent _asfirst_person_character) (Variables|Default|GetSecondsOfBoost))
  (bind _asbeanbag_game_mode (Utilities|Casting|CastToBeanbagGameMode (Game|GetGameMode)))
  (bind _output_get (Variables|/Game/Blueprints/BeanbagGameMode.BeanbagGameMode_C|SetSpawnTransform _asbeanbag_game_mode (Math|Transform|MakeTransform (.location _returnvalue) (.rotation _returnvalue) "1,1,1")))
  (if (== _output_get (Variables|/Game/Blueprints/BeanbagGameMode.BeanbagGameMode_C|GetSpawnTransform _asbeanbag_game_mode))
    (Rendering|SetVisibility (Variables|Default|GetParticleSystem) true false)
    (else
      (Rendering|SetVisibility (Variables|Default|GetParticleSystem) false false))))

(event EventTick
  (params (DeltaSeconds :type Float%20%28single-precision%29))
  (bind _asbeanbag_game_mode (Utilities|Casting|CastToBeanbagGameMode (Game|GetGameMode)))
  (if (== (Transformation|GetWorldTransform (Variables|Default|GetArrow)) (Variables|/Game/Blueprints/BeanbagGameMode.BeanbagGameMode_C|GetSpawnTransform _asbeanbag_game_mode))
    (Development|SetHiddeninGame (Variables|Default|GetParticleSystem) false false)
    (else
      (Development|SetHiddeninGame (Variables|Default|GetParticleSystem) true false))))

(fn ConstructionScript)